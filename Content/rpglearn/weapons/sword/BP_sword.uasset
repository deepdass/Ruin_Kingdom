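; BP_sword is a melee weapon that deals point damage through traces while activated by its functionality events.
; Each tick, it sphere-traces from the previous to current positions of points interpolated between two blade markers, covering the swept arc between frames.
; Each actor is hit once per activation, spawning a Niagara effect at impact.
; The holder, set from the parent actor or pickup event, is ignored and credited as instigator.
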(event EventBeginPlay
  (bind _returnvalue (Actor|GetParentActor))
  (Utilities|IsValid _returnvalue
    (:Is%20Valid
      (CallFunction|PickedUp _returnvalue))))

(event EventPickthisup
  (params (actorthatpickedthisup :type Actor%20Object%20Reference))
  (CallFunction|PickedUp actorthatpickedthisup))

(event EventTick
  (params (DeltaSeconds :type Float%20%28single-precision%29))
  (bind _numberofcollisionpoints (Variables|Weapon|Getnumberofcollisionpoints))
  (bind _returnvalue (- _numberofcollisionpoints 1))
  (if (Variables|Default|Getshoulddotracingfordamage)
    (for _index (range 0 _returnvalue)
      (bind (_outhits _returnvalue_2) (Collision|MultiSphereTraceForObjects (Utilities|Array|Get(acopy) (Variables|Default|Getpreviouslocationarray) _index) (Math|Vector|Lerp(Vector) (Transformation|GetWorldLocation (Variables|Default|Getbaseswordlocation)) (Transformation|GetWorldLocation (Variables|Default|Getbaseswordlocation1)) (/ _index _returnvalue)) (Variables|weapon|GetRadius) (Utilities|Array|MakeArray "ObjectTypeQuery2" "ObjectTypeQuery3") false (Variables|Default|Getactorhitted) (Variables|Weapon|GetDraw%20Debug%20Type)))
      (Utilities|FlowControl|Sequence
        (:then_0
          (if _returnvalue_2
            (for _array_element _outhits
              (bind _returnvalue_3 (Utilities|Array|AddUnique (Variables|Default|Getactorhitted) (.HitActor (Collision|BreakHitResult _array_element))))
              (if (>= _returnvalue_3 0)
                (Game|Damage|ApplyPointDamage (.HitActor (Collision|BreakHitResult _array_element)) (Variables|weapon|GetBase%20Damage) (Math|Vector|GetUnitDirection(Vector) (.TraceStart (Collision|BreakHitResult _array_element)) (.TraceEnd (Collision|BreakHitResult _array_element))) _array_element (Game|GetInstigatorController (Variables|Default|Getactorholdingitref)) self)
                (Niagara|SpawnSystematLocation (Variables|Default|GetSystem%20Template) (.Location (Collision|BreakHitResult _array_element)) (Math|Conversions|RotationFromXVector (Math|Vector|GetUnitDirection(Vector) (.TraceStart (Collision|BreakHitResult _array_element)) (.TraceEnd (Collision|BreakHitResult _array_element)))))))))
        (:then_1
          (Utilities|Array|SetArrayElem (Variables|Default|Getpreviouslocationarray) _index (Math|Vector|Lerp(Vector) (Transformation|GetWorldLocation (Variables|Default|Getbaseswordlocation)) (Transformation|GetWorldLocation (Variables|Default|Getbaseswordlocation1)) (/ _index _returnvalue))))))))

(event EventDeactivateobjectfunctionality
  (Variables|Default|Setshoulddotracingfordamage false))

(event EventActivateobjectfunctionality
  (bind _actorhitted (Variables|Default|Getactorhitted))
  (bind _numberofcollisionpoints (Variables|Weapon|Getnumberofcollisionpoints))
  (bind _returnvalue (- _numberofcollisionpoints 1))
  (Variables|Default|Setshoulddotracingfordamage true)
  (Utilities|Array|Clear _actorhitted)
  (Utilities|Array|Add _actorhitted (Variables|Default|Getactorholdingitref))
  (Utilities|Array|Clear (Variables|Default|Getpreviouslocationarray))
  (for _index (range 0 _returnvalue)
    (Utilities|Array|Add (Variables|Default|Getpreviouslocationarray) (Math|Vector|Lerp(Vector) (Transformation|GetWorldLocation (Variables|Default|Getbaseswordlocation)) (Transformation|GetWorldLocation (Variables|Default|Getbaseswordlocation1)) (/ _index _returnvalue)))))

(fn ConstructionScript)

(fn PickedUp
  (params (actorthatpickedup :type Actor%20Object%20Reference))
  (Variables|Default|Setactorholdingitref actorthatpickedup))