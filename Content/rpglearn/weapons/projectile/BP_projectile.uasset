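; Projectile actor for the RPG's weapons that deals point damage to whatever it hits.
; On BeginPlay its collision sphere ignores the instigator while moving.
; When ProjectileMovement stops, it applies ProjectileDamage to the hit actor on behalf of the instigator's controller, spawns the Spell effect system at the impact point, then destroys itself.
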(event OnProjectileStop(ProjectileMovement)
  (params (ImpactResult :type Hit%20Result%20Structure%20%28by%20ref%29))
  (bind (_bblockinghit _binitialoverlap _time _distance _location _impactpoint _normal _impactnormal _physmat _hitactor) (Collision|BreakHitResult ImpactResult))
  (Utilities|FlowControl|Sequence
    (:then_0
      (Game|Damage|ApplyPointDamage _hitactor (Variables|Default|GetprojectileDamage) (Math|Vector|GetUnitDirection(Vector) (Transformation|GetActorLocation) (Transformation|GetActorLocation _hitactor)) ImpactResult (Game|GetInstigatorController) self)
      (Niagara|SpawnSystematLocation (Variables|Default|GetSpell) _impactpoint (Math|Conversions|RotationFromXVector (Transformation|GetActorForwardVector))))
    (:then_1
      (Actor|DestroyActor))))

(event EventBeginPlay
  (Collision|IgnoreActorwhenMoving (Variables|Default|GetSpherecollision) (Game|GetInstigator) true))

(event Collision|EventActorBeginOverlap
  (params (OtherActor :type Actor%20Object%20Reference)))

(event EventTick
  (params (DeltaSeconds :type Float%20%28single-precision%29)))

(fn ConstructionScript)