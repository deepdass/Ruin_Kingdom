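; GM_rpg is the RPG game mode, handling player spawning in a World Partition level and the win screen.
; On BeginPlay, a looping timer polls the World Partition subsystem until all streaming completes, then clears itself and restarts the first player controller's player.
; A wincondition event creates the WB_winscreen widget, adds it to the viewport and switches input to UI only, with focus on the retry button.
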(event Custom|win%20condition
  (bind _returnvalue (UserInterface|CreateWidget "/Game/rpglearn/player/ui/WB_winscreen.WB_winscreen_C"))
  (Input|SetInputModeUIOnly (Game|GetPlayerController 0) (Variables|/Game/rpglearn/player/ui/WB_winscreen.WB_winscreen_C|GetBTN_retry _returnvalue) "DoNotLock" false)
  (UserInterface|Viewport|AddtoViewport _returnvalue 0))

(event Custom|checkstreaming
  (bind _returnvalue (Streaming|IsAllStreamingCompleted (WorldSubsystems|GetWorldPartitionSubsystem)))
  (if _returnvalue
    (Utilities|Time|ClearandInvalidateTimerbyHandle (Variables|Default|Getstreamingchecktimer))
    (Class|GameModeBase|RestartPlayer (Game|GetPlayerController 0))))

(event EventBeginPlay
  (bind _returnvalue (Utilities|Time|SetTimerbyEvent (delegate Custom|checkstreaming) 0.1 true))
  (Variables|Default|Setstreamingchecktimer _returnvalue))

(event EventTick
  (params (DeltaSeconds :type Float%20%28single-precision%29)))

(fn ConstructionScript)