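; Player HUD Blueprint that puts the WB_hud widget on screen and hooks it up to the controlled pawn's character info.
; On BeginPlay it listens for the owning controller's possessed pawn changes, creating and adding a new WB_hud each time without removing the previous one.
; It then binds the health-change and damage-received dispatchers on the pawn's BPC_characterinfo and calls Sethealth with the current Health value.
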(event Custom|OnPossessedPawnChanged_Event
  (params (OldPawn :type Pawn%20Object%20Reference) (NewPawn :type Pawn%20Object%20Reference))
  (bind _returnvalue (Game|Player|GetOwningPlayerController))
  (bind _returnvalue_2 (Pawn|GetControlledPawn _returnvalue))
  (bind _returnvalue_3 (Actor|GetComponentbyClass _returnvalue_2 "/Game/rpglearn/characters/global/BPC_characterinfo.BPC_characterinfo_C"))
  (bind _returnvalue_4 (UserInterface|CreateWidget "/Game/rpglearn/player/ui/WB_hud.WB_hud_C"))
  (Variables|Default|Sethudwref _returnvalue_4)
  (UserInterface|Viewport|AddtoViewport (Variables|Default|Gethudwref) 0)
  (Utilities|IsValid _returnvalue
    (:Is%20Valid
      (Utilities|IsValid _returnvalue_2
        (:Is%20Valid
          (EventDispatchers|BindEventtoOnhealthchange _returnvalue_3 (EventDispatchers|CreateEvent (Variables|/Game/rpglearn/player/ui/WB_hud.WB_hud_C|GetWBC_healthbar (Variables|Default|Gethudwref)) :!event Setnewhealth))
          (EventDispatchers|BindEventtoOndamagereceive _returnvalue_3 (EventDispatchers|CreateEvent (Variables|Default|Gethudwref) :!event Enemyhitflash))
          (Default|Sethealth _returnvalue_3 (Variables|/Game/rpglearn/characters/global/BPC_characterinfo.BPC_characterinfo_C|Gethealth _returnvalue_3)))))))

(event EventBeginPlay
  (EventDispatchers|AssignOnPossessedPawnChanged (Game|Player|GetOwningPlayerController) (delegate Custom|OnPossessedPawnChanged_Event)))

(fn ConstructionScript)