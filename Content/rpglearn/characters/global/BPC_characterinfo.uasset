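; Character info component that gives its owning actor team-based health, damage and death handling.
; On BeginPlay it binds to the owner's damage events; any damage from a different team lowers health, fires a damage-received event and plays a world camera shake.
; Health changes are clamped and broadcast through dispatchers, with a death event at zero, while the point damage handler is left empty.
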(event Custom|OnTakeAnyDamage_Event
  (params (DamagedActor :type Actor%20Object%20Reference) (Damage :type Float%20%28single-precision%29) (DamageType :type Damage%20Type%20Object%20Reference) (InstigatedBy :type Controller%20Object%20Reference) (DamageCauser :type Actor%20Object%20Reference))
  (bind _returnvalue (Pawn|GetControlledPawn InstigatedBy))
  (if (Utilities|Enum|NotEqual(Enum) (Variables|BPC_characterinfo_C|Getteam (Actor|GetComponentbyClass DamagedActor "BPC_characterinfo_C")) (Variables|BPC_characterinfo_C|Getteam (Actor|GetComponentbyClass _returnvalue "BPC_characterinfo_C")))
    (bind _actualdamagerecieve (CallFunction|Dodamage Damage))
    (Default|CallOndamagereceive _actualdamagerecieve _returnvalue)
    (Camera|PlayWorldCameraShake "/Game/rpglearn/player/camerashake/CS_onhit.CS_onhit_C" (Transformation|GetActorLocation (Components|GetOwner)) 3e+02 3e+02)))

(event Custom|OnTakePointDamage_Event
  (params (DamagedActor :type Actor%20Object%20Reference) (Damage :type Float%20%28single-precision%29) (InstigatedBy :type Controller%20Object%20Reference) (HitLocation :type Vector) (FHitComponent :type Primitive%20Component%20Object%20Reference) (BoneName :type Name) (ShotFromDirection :type Vector) (DamageType :type Damage%20Type%20Object%20Reference) (DamageCauser :type Actor%20Object%20Reference)))

(event EventBeginPlay
  (bind _returnvalue (Components|GetOwner))
  (EventDispatchers|AssignOnTakeAnyDamage _returnvalue (EventDispatchers|CreateEvent :!event Custom|OnTakeAnyDamage_Event))
  (EventDispatchers|AssignOnTakePointDamage _returnvalue (EventDispatchers|CreateEvent :!event Custom|OnTakePointDamage_Event)))

(event EventTick
  (params (DeltaSeconds :type Float%20%28single-precision%29)))

(fn Sethealth
  (params (newhealth :type Float%20%28double-precision%29))
  (bind _maxhealth (Variables|Default|Getmaxhealth))
  (bind _output_get (Variables|Default|Sethealth (Math|Float|Clamp(Float) newhealth 0.0 _maxhealth)))
  (Default|CallOnhealthchange _output_get _maxhealth)
  (if (<= _output_get 0.0)
    (CallFunction|Death)))

(fn Refillhealth
  (CallFunction|Sethealth (Variables|Default|Getmaxhealth)))

(fn Dodamage
  (params (damagerec :type Float%20%28double-precision%29))
  (CallFunction|Sethealth (- (Variables|Default|Gethealth) damagerec))
  (return damagerec))

(fn Ischaracterdead
  (return (<= (Variables|Default|Gethealth) 0.0)))

(fn Death
  (Default|CallOndeath))