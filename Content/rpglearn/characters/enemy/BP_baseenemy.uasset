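; BP_baseenemy is a base enemy character that reacts to damage and death through its character info component.
; The component's health is refilled on BeginPlay.
; Taking damage writes the instigator's location to the AI controller's "locationtosearch" blackboard key.
; On death, capsule collision is disabled and the mesh switches to the PhysicsActor profile with simulated physics, producing a ragdoll.
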(event Ondeath(BPC_characterinfo)
  (bind _mesh (Variables|Character|GetMesh))
  (Collision|SetCollisionEnabled (Variables|Collision|GetCapsuleComponent) "NoCollision")
  (Collision|SetCollisionProfileName _mesh "PhysicsActor" true :!class /Script/Engine.PrimitiveComponent)
  (Physics|SetSimulatePhysics _mesh true))

(event Ondamagereceive(BPC_characterinfo)
  (params (damagerecie :type Float%20%28double-precision%29) (instigator :type Actor%20Object%20Reference))
  (AI|Components|Blackboard|SetValueasVector (AI|GetBlackboard (Pawn|GetController)) (Utilities|Name|MakeLiteralName "locationtosearch") (Transformation|GetActorLocation instigator)))

(event EventBeginPlay
  (Default|Refillhealth (Variables|Default|GetBPC_characterinfo)))

(fn ConstructionScript)