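; BP_reward is an interactable reward pickup in the RPG that triggers the game's win condition when collected.
; Entering its sphere shows a text label, turned toward player 0 each tick while visible, and registers the actor in the RPG character's interactable list; leaving hides and unregisters it.
; Interaction calls the GM_rpg game mode's WinCondition, then destroys the actor.
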(event OnComponentBeginOverlap(Sphere)
  (params (OverlappedComponent :type Primitive%20Component%20Object%20Reference) (OtherActor :type Actor%20Object%20Reference) (OtherComp :type Primitive%20Component%20Object%20Reference) (OtherBodyIndex :type Integer) (bFromSweep :type Boolean) (SweepResult :type Hit%20Result%20Structure%20%28by%20ref%29))
  (Rendering|SetVisibility (Variables|Default|Getreward%20text) true false)
  (bind _asbp_rpgcharacter (Utilities|Casting|CastToBP_rpgcharacter OtherActor))
  (Default|Addinteractableobjectinrange _asbp_rpgcharacter self))

(event OnComponentEndOverlap(Sphere)
  (params (OverlappedComponent :type Primitive%20Component%20Object%20Reference) (OtherActor :type Actor%20Object%20Reference) (OtherComp :type Primitive%20Component%20Object%20Reference) (OtherBodyIndex :type Integer))
  (Rendering|SetVisibility (Variables|Default|Getreward%20text) false false)
  (bind _asbp_rpgcharacter (Utilities|Casting|CastToBP_rpgcharacter OtherActor))
  (Default|Removeinteractableobject _asbp_rpgcharacter self))

(event Custom|getreward
  (bind _asgm_rpg (Utilities|Casting|CastToGM_rpg (Game|GetGameMode)))
  (Default|WinCondition _asgm_rpg)
  (Actor|DestroyActor))

(event Collision|EventActorBeginOverlap
  (params (OtherActor :type Actor%20Object%20Reference)))

(event EventTick
  (params (DeltaSeconds :type Float%20%28single-precision%29))
  (bind _reward_text (Variables|Default|Getreward%20text))
  (if (Variables|/Script/Engine.SceneComponent|GetbVisible (Variables|Default|Getreward%20text))
    (Transformation|SetWorldRotation _reward_text (Math|Rotator|FindLookatRotation (Transformation|GetWorldLocation _reward_text) (Transformation|GetActorLocation (Game|GetPlayerCharacter 0))) false false)))

(event EventInteractionwithobject
  (CallFunction|Getreward))

(fn ConstructionScript)